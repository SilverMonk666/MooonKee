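; BP_loot is a weapon-upgrade pickup that grants the first-person character a fire mode chosen by its Type enum.
; On BeginPlay, a text render component displays the Type name as a label.
; When BP_FirstPersonCharacter triggers its Hit event, it sets the Bomb flag for Cluster-Fire or FullAUto for Full-Auto-Fire, then destroys itself.
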(event `self.ReceiveHit`
  (params (MyComp :type "PrimitiveComponent Object Reference") (Other :type "Actor Object Reference") (OtherComp :type "PrimitiveComponent Object Reference") (bSelfMoved :type Boolean) (HitLocation :type "Vector Structure") (HitNormal :type "Vector Structure") (NormalImpulse :type "Vector Structure") (Hit :type "HitResult Structure (by ref)"))
  (bind _asbp_first_person_character (cast `/Game/FirstPerson/Blueprints/BP_FirstPersonCharacter` Other))
  (switch `/Game/Bluepriunt/LootTypes` (`self.Type`)
    (:`NewEnumerator0`
      (set `/Game/FirstPerson/Blueprints/BP_FirstPersonCharacter.Bomb` true _asbp_first_person_character))
    (:`NewEnumerator1`
      (set `/Game/FirstPerson/Blueprints/BP_FirstPersonCharacter.Full AUto` true _asbp_first_person_character)))
  (`self.K2_DestroyActor`))

(event `self.ReceiveBeginPlay`
  (`TextRenderComponent.K2_SetText` (`self.TextRender`) (`KismetTextLibrary.Conv_StringToText` (`|GetEnumeratorNameAsString` (`self.Type`)))))

(fn `UserConstructionScript`)