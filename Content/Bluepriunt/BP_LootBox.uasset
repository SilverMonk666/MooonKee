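; Loot box that is meant to swing open, spawn random loot and close when the first-person character enters its zone.
; A timeline drives the Scene component's roll, with a First flag picking the sign.
; On finish, a FlipFlop alternates between spawning BP_loot with delayed reversal and resetting that flag.
; Rotation is noted as broken: clamps follow the 90-degree scaling with bounds within one degree of zero.
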(event `self.Open Zone.OnComponentBeginOverlap`
  (params (OverlappedComponent :type "PrimitiveComponent Object Reference") (OtherActor :type "Actor Object Reference") (OtherComp :type "PrimitiveComponent Object Reference") (OtherBodyIndex :type Integer) (bFromSweep :type Boolean) (SweepResult :type "HitResult Structure (by ref)"))
  (bind _scene (`self.Scene`))
  (bind (_relativerotation_roll _relativerotation_pitch _relativerotation_yaw) (`KismetMathLibrary.BreakRotator` (`SceneComponent.RelativeRotation` _scene)))
  ;[1 1 1] Rotate And spawn loot (THE ROTATION DOESNT WORK IDK WHY I WANT IT TO OPEN 90 DEGREES THEN CLOSE!!!)
  (cast `/Game/FirstPerson/Blueprints/BP_FirstPersonCharacter` OtherActor)
  (`|ExecutionSequence`
    (:`then_0`
      (`/Engine/EditorBlueprintResources/StandardMacros.DoOnce` false :!label _label
        (:`Completed`
          (bind (_direction _rotation) (`Timeline|Rotation` :!via `PlayFromStart` :!label _label_2)
            (:`Update`
              (bind _returnvalue (* _rotation 90.0))
              (`KismetSystemLibrary.PrintString` (`KismetStringLibrary.Conv_DoubleToString` _returnvalue) true true (struct :`R` 1.0 :`A` 1.0) 70.0)
              (if (`self.First`)
                (`SceneComponent.K2_SetRelativeRotation` _scene (`KismetMathLibrary.MakeRotator` (`KismetMathLibrary.FClamp` (* _returnvalue -1.0) 0.0 -1.0) _relativerotation_pitch _relativerotation_yaw) false false)
                (else
                  (`SceneComponent.K2_SetRelativeRotation` _scene (`KismetMathLibrary.MakeRotator` (`KismetMathLibrary.FClamp` _returnvalue 0.0 1.0) _relativerotation_pitch _relativerotation_yaw) false false))))
            (:`Finished`
              (`/Engine/EditorBlueprintResources/StandardMacros.FlipFlop`
                (:`A`
                  (bind _output_get (set `self.NewVar` (cast `/Game/Bluepriunt/LootTypes` (`KismetMathLibrary.Conv_IntToByte` (`KismetMathLibrary.RandomIntegerInRange` 0 1)))))
                  (`|SpawnActorFromClass` "/Game/Bluepriunt/BP_loot.BP_loot_C" (`KismetMathLibrary.MakeTransform` (`SceneComponent.K2_GetComponentLocation` (`self.SpawnPoint`))) "Undefined" "MultiplyWithRoot" null _output_get null)
                  (set `self.First` false)
                  (`KismetSystemLibrary.PrintString` (`|GetEnumeratorNameAsString` (`self.NewVar`)))
                  (`KismetSystemLibrary.Delay` 40.0)
                  (goto _label_2 :!via `ReverseFromEnd`))
                (:`B`
                  (set `self.First` true))))))))
    (:`then_1`
      (`KismetSystemLibrary.Delay` 1.0)
      (goto _label :!via `Reset`))))

(fn `UserConstructionScript`)