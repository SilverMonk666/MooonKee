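; BP_BigJohnson is an enemy that chases the player, re-issuing AIMoveTo every Tick.
; Projectile hits lower its Health, and the killing shot awards the player score and health before destroying it.
; Hitting the player either kills them at exactly 1 Health or subtracts 3 and destroys the enemy.
; A separate Die event adds an explosion effect and sound, but nothing in this graph calls it.
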(event `self.ReceiveTick`
  (params (DeltaSeconds :type "Float (single-precision)"))
  (`|AIMoveTo` self (0.0 0.0 0.0) (`GameplayStatics.GetPlayerCharacter` 0)))

(event `self.ReceiveHit`
  (params (MyComp :type "PrimitiveComponent Object Reference") (Other :type "Actor Object Reference") (OtherComp :type "PrimitiveComponent Object Reference") (bSelfMoved :type Boolean) (HitLocation :type "Vector Structure") (HitNormal :type "Vector Structure") (NormalImpulse :type "Vector Structure") (Hit :type "HitResult Structure (by ref)"))
  (bind _health (`self.health`))
  (cast `/Game/FirstPerson/Blueprints/BP_FirstPersonProjectile` Other
    (:`then`
      (if (== _health 1)
        (bind _returnvalue (`GameplayStatics.GetActorOfClass` "/Game/FirstPerson/Blueprints/BP_FirstPersonCharacter.BP_FirstPersonCharacter_C"))
        (`/Game/FirstPerson/Blueprints/BP_FirstPersonCharacter.Add Score` _returnvalue)
        (`/Game/FirstPerson/Blueprints/BP_FirstPersonCharacter.Add Health` _returnvalue 1)
        (`self.K2_DestroyActor`)
        (else
          (bind _output_get (set `self.health` (- _health 1)))
          (`KismetSystemLibrary.PrintString` (`KismetStringLibrary.Conv_IntToString` _output_get)))))
    (:`CastFailed`
      (bind _asbp_first_person_character (cast `/Game/FirstPerson/Blueprints/BP_FirstPersonCharacter` Other))
      (bind _health_2 (`/Game/FirstPerson/Blueprints/BP_FirstPersonCharacter.health` _asbp_first_person_character))
      (if (== _health_2 1)
        (`/Game/FirstPerson/Blueprints/BP_FirstPersonCharacter.Kill` _asbp_first_person_character)
        (else
          (set `/Game/FirstPerson/Blueprints/BP_FirstPersonCharacter.health` (- _health_2 3) _asbp_first_person_character)
          (`self.K2_DestroyActor`))))))

(event `Die`
  (bind _returnvalue (`self.K2_GetActorLocation`))
  (`GameplayStatics.SpawnEmitterAtLocation` "/Game/StarterContent/Particles/P_Explosion.P_Explosion" _returnvalue)
  (`GameplayStatics.PlaySoundAtLocation` "/Game/StarterContent/Audio/Explosion01.Explosion01" _returnvalue (struct) 1.0 1.0 0.0 "/Game/Audio/johnsonbig.johnsonbig" null null null)
  (`self.K2_DestroyActor`))

(fn `UserConstructionScript`)